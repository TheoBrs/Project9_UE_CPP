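; BP_RunGameMode is a game mode that keeps a running track of floor tiles going by spawning and recycling BP_FloorTile actors.
; On BeginPlay it spawns an initial batch, chaining each tile to the previous one through its AttachTransform and binding to its Exited event.
; When a tile is exited, it destroys that tile after a short delay and spawns a new one at the end of the chain.
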(event `self.ReceiveBeginPlay`
  (for _ (range 7)
    (`self.SpawnTile`)))

(event `OnTileExited`
  (params (FloorTile :type "/Game/Components/BP_FloorTile Object Reference"))
  (`KismetSystemLibrary.Delay` 0.3)
  (`self.K2_DestroyActor` FloorTile)
  (`self.SpawnTile`))

(fn `SpawnTile`
  (bind _returnvalue (`|SpawnActorFromClass` "/Game/Components/BP_FloorTile.BP_FloorTile_C" (`self.TileAttachTransform`) "Undefined" "MultiplyWithRoot" null null))
  (set `self.TileAttachTransform` (`/Game/Components/BP_FloorTile.AttachTransform` _returnvalue))
  (add `/Game/Components/BP_FloorTile.Exited` _returnvalue (`|CreateDelegate` :!event `OnTileExited`))
  (return))

(fn `UserConstructionScript`)