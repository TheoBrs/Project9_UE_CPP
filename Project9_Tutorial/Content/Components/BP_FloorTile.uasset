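; Floor tile actor that spawns a random obstacle on itself and signals when the player reaches its end.
; On BeginPlay it picks a class from ObstacleTypes, spawns it at a random point in a fixed box, then attaches it with KeepRelative so that point becomes tile-local.
; GetAttachTransform exposes the AttachPoint world transform.
; Player pawn overlap with TileEndBox fires the Exited dispatcher, passing the tile.
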(event `self.ReceiveBeginPlay`
  (`self.SpawnObstacle`)
  (`self.GetAttachTransform`))

(event `self.TileEndBox.OnComponentBeginOverlap`
  (params (OverlappedComponent :type "PrimitiveComponent Object Reference") (OtherActor :type "Actor Object Reference") (OtherComp :type "PrimitiveComponent Object Reference") (OtherBodyIndex :type Integer) (bFromSweep :type Boolean) (SweepResult :type "HitResult Structure (by ref)"))
  (if (== OtherActor (`GameplayStatics.GetPlayerPawn` 0))
    (`self.Exited` self)))

(fn `GetAttachTransform`
  (returns (AttachTransform :type "Transform Structure"))
  (bind _output_get (set `self.AttachTransform` (`SceneComponent.K2_GetComponentToWorld` (`self.AttachPoint`))))
  (return _output_get))

(fn `SpawnObstacle`
  (bind _returnvalue (`|SpawnActorFromClass` (`KismetArrayLibrary.Array_Random` (`self.ObstacleTypes`)) (`KismetMathLibrary.Conv_VectorToTransform` (`KismetMathLibrary.RandomPointInBoundingBox` (700.0 0.0 5.0) (50.0 400.0 2.0))) "Undefined" "MultiplyWithRoot" null null))
  (`self.K2_AttachToActor` _returnvalue self "None" "KeepRelative" "KeepRelative" "KeepRelative" true))

(fn `UserConstructionScript`)